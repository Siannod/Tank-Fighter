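; BP_Checkpoint is a one-shot checkpoint trigger that updates the player's spawn point.
; On the first BP_PlayerCharacter overlap with its box, it deactivates and stores its location as SpawnPoint on BP_MechPlayerController.
; It then spawns a WBP_PickUpNotification at that location displaying "Checkpoint!".
; Every player overlap also assigns MaxHealth to itself, which restores no health as written.
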(event `self.Box.OnComponentBeginOverlap`
  (params (OverlappedComponent :type "PrimitiveComponent Object Reference") (OtherActor :type "Actor Object Reference") (OtherComp :type "PrimitiveComponent Object Reference") (OtherBodyIndex :type Integer) (bFromSweep :type Boolean) (SweepResult :type "HitResult Structure (by ref)"))
  (bind _returnvalue_location (`KismetMathLibrary.BreakTransform` (`self.GetTransform`)))
  ;[1 1 1] Checkpoint Overlap - UI notification and Spawn Loc update
  (bind _asbp_player_character (cast `/Game/Blueprints/BP_PlayerCharacter` OtherActor))
  (set `/Game/Blueprints/BP_PlayerCharacter.MaxHealth` (`/Game/Blueprints/BP_PlayerCharacter.MaxHealth` _asbp_player_character) _asbp_player_character)
  (if (`self.Active`)
    (set `self.Active` false) ; Disable this Checkpoint\nso it cannot be continually\nused
    (bind _asbp_mech_player_controller (cast `/Game/Blueprints/MiscBlueprints/BP_MechPlayerController` (`GameplayStatics.GetPlayerController` 0)))
    (set `/Game/Blueprints/MiscBlueprints/BP_MechPlayerController.SpawnPoint` (`self.K2_GetActorLocation`) _asbp_mech_player_controller)
    (`|SpawnActorFromClass` "/Game/UI/WBP_PickUpNotification.WBP_PickUpNotification_C" (`KismetMathLibrary.MakeTransform` _returnvalue_location) "AlwaysSpawn" "SelectDefaultAtRuntime" null "Checkpoint!" null) ; Spawn a UI notification at the Checkpoint Location\nTell it to display 'Checkpoint!'
  ))

(fn `UserConstructionScript`)