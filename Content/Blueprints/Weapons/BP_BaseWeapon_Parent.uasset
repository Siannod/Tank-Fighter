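; Base weapon Blueprint for a tank, whose Initiate event stores the tank reference and passes it the weapon's name and mesh to load.
; Empty primary and secondary events mirror Enhanced Input trigger states, as hooks for child weapons to fill in.
; Ammo fills to max on BeginPlay, CheckReload reports when it is empty, and a helper plays camera shakes.
; The reload input only prints a debug string.
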(event `Initiate`
  (params (TankREF :type "/Game/Blueprints/BP_PlayerCharacter Object Reference"))
  (bind _output_get (set `self.MyTank` TankREF))
  (`/Game/Blueprints/BP_PlayerCharacter.LoadNewWeapon` _output_get (`self.WeaponName`) (`self.WeaponMesh`)))

(event `Triggered`
  ;[1 1 1] Triggered - Fires on Tick whilst key is down
)

(event `TriggeredSEC`)

(event `StartedSEC`)

(event `Started`
  ;[1 1 1] Started - Fires once when the key is first pressed
)

(event `OngoingSEC`)

(event `CancelledSEC`)

(event `Completed`
  ;[1 1 1] Completed - When the key is released
)

(event `CompletedSEC`)

(event `Ongoing`)

(event `self.ReceiveBeginPlay`
  (set `self.CurrentAmmo` (`self.MaxAmmo`)))

(event `Cancelled`)

(event `EnhancedInput|/Game/Blueprints/MiscBlueprints/IA_Reload`
  (params (ActionValue :type Boolean) (ElapsedSeconds :type "Float (double-precision)") (TriggeredSeconds :type "Float (double-precision)") (InputAction :type "InputAction Object Reference" :default "/Game/Blueprints/MiscBlueprints/IA_Reload.IA_Reload"))
  (:`Triggered`
    (`KismetSystemLibrary.PrintString` "Hello")))

(fn `CameraShake`
  (params (`CameraShake Class` :type "/Game/StudentWork/Weapon/BP_cameraShake Class Reference") (Scale :type "Float (double-precision)" :default 1.0))
  (`PlayerCameraManager.StartCameraShake` :`self` (`GameplayStatics.GetPlayerCameraManager` 0) :`ShakeClass` `CameraShake Class` :`Scale` Scale))

(fn `CheckReload`
  (returns (NoAmmo :type Boolean))
  (`/Engine/EditorBlueprintResources/StandardMacros.CompareInt` (`self.CurrentAmmo`)
    (:`>`
      (return false))
    (:`==`
      _)
    (:`<`
      _))
  (return true))

(fn `UserConstructionScript`)