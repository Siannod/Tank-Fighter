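; Tank weapon Blueprint, filed under inactive old weapons, that fires exploding projectiles.
; When triggered off cooldown, it spawns BP_exploding_projectile at the location and rotation of the owning tank's direction arrow.
; A boolean gate, cleared by a short timer event, limits the fire rate.
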(event `self.Triggered`
  (bind _directionarrow (`/Game/Blueprints/BP_PlayerCharacter.DirectionArrow` (`self.MyTank`)))
  (if (not (`self.Cooldown_0`))
    (`|SpawnActorFromClass` "/Game/INACTIVE/OldWeapons/Projectiles/BP_exploding_projectile.BP_exploding_projectile_C" (`KismetMathLibrary.MakeTransform` (`SceneComponent.K2_GetComponentLocation` _directionarrow) (`SceneComponent.K2_GetComponentRotation` _directionarrow)) "Undefined" "MultiplyWithRoot" null null)
    (set `self.Cooldown_0` true)
    (`KismetSystemLibrary.K2_SetTimerDelegate` (delegate `End Cooldown`) 0.1)))

(event `End Cooldown`
  (set `self.Cooldown_0` false))

(fn `UserConstructionScript`
  (`parent.UserConstructionScript`))