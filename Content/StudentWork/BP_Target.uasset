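; BP_Target is a damageable target that flashes when hit, then explodes.
; The construction script creates a dynamic flash material on its mesh.
; The first damage event, gated by a DoOnce, plays a timeline that drives the material's FlashLevel parameter.
; When the timeline finishes, it applies radial damage around its centre and destroys itself, so nearby targets can chain-react.
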(event `self.ReceiveAnyDamage`
  (params (Damage :type "Float (single-precision)") (DamageType :type "DamageType Object Reference") (InstigatedBy :type "Controller Object Reference") (DamageCauser :type "Actor Object Reference"))
  (`/Engine/EditorBlueprintResources/StandardMacros.DoOnce` false
    (:`Completed`
      (bind (_direction _flash) (`Timeline|Flash` :!via `PlayFromStart`)
        (:`Update`
          (`MaterialInstanceDynamic.SetScalarParameterValue` (`self.Flash Material`) "FlashLevel" _flash))
        (:`Finished`
          (`GameplayStatics.ApplyRadialDamage` :`BaseDamage` 10.0 :`Origin` (`SceneComponent.K2_GetComponentLocation` (`self.centre`)) :`DamageRadius` 200.0 :`DamageCauser` null :`InstigatedByController` null :`bDoFullDamage` true)
          (`self.K2_DestroyActor`))))))

(fn `UserConstructionScript`
  (bind _returnvalue (`PrimitiveComponent.CreateDynamicMaterialInstance` (`self.StaticMesh`) 0 "/Game/StudentWork/M_controlledFlash.M_controlledFlash" "None"))
  (set `self.Flash Material` _returnvalue))