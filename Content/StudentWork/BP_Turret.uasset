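; Stationary enemy turret that fires projectile bursts indefinitely and can be destroyed by damage.
; A looping timer starts each burst, and a faster nested timer spawns three BP_enemy_projectile actors from the Arrow's transform.
; The burst timer's clear branch needs a count above three, which is never reached, so it idles until the next burst.
; Damage lowers health and plays a timeline-driven dynamic-material flash, destroying the turret afterwards at zero health.
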(event `self.ReceiveBeginPlay`
  ; Fires indefinetly
  (bind _output_get (set `self.maxHealth` 100))
  (set `self.currentHealth` _output_get)
  (bind _returnvalue (`KismetSystemLibrary.K2_SetTimerDelegate` (delegate `Fire Burst`) 2.0 true))
  (set `self.Turret Counter` _returnvalue))

(event `Fire Burst`
  ; Controls a round
  (set `self.projectileCounter` 0)
  (bind _returnvalue (`KismetSystemLibrary.K2_SetTimerDelegate` (delegate `burst`) 0.1 true))
  (set `self.burstTimer` _returnvalue))

(event `burst`
  (bind _arrow (`self.Arrow`))
  ; Individual bullet
  (`/Engine/EditorBlueprintResources/StandardMacros.CompareInt` (`self.projectileCounter`) 3
    (:`>`
      (`KismetSystemLibrary.K2_ClearAndInvalidateTimerHandle` (`self.burstTimer`)))
    (:`<`
      (`|SpawnActorFromClass` "/Game/StudentWork/Weapon/OldWeapons/Projectiles/BP_enemy_projectile.BP_enemy_projectile_C" (`KismetMathLibrary.MakeTransform` (`SceneComponent.K2_GetComponentLocation` _arrow) (`SceneComponent.K2_GetComponentRotation` _arrow)) "Undefined" "MultiplyWithRoot" null null)
      (set `self.projectileCounter` (+ (`self.projectileCounter`) 1)))))

(event `self.ReceiveAnyDamage`
  (params (Damage :type "Float (single-precision)") (DamageType :type "DamageType Object Reference") (InstigatedBy :type "Controller Object Reference") (DamageCauser :type "Actor Object Reference"))
  ;[0.15 0.025 0.025 0.5] Take Damage
  (bind _output_get (set `self.currentHealth` (`KismetMathLibrary.FTrunc` (- (`self.currentHealth`) Damage))))
  ;[0.15 0.02031 0.02031 0.5] Change Colour
  (bind (_direction _flash_track) (`Timeline|Flash` :!via `PlayFromStart`)
    (:`Update`
      (`MaterialInstanceDynamic.SetScalarParameterValue` (`self.FlashMaterial`) "FlashLevel" _flash_track))
    (:`Finished`
      (if (<= _output_get 0)
        (`self.K2_DestroyActor`)))))

(fn `UserConstructionScript`
  (locals (NewLocalVar :type "StaticMeshComponent Object Reference"))
  (bind _returnvalue (`PrimitiveComponent.CreateDynamicMaterialInstance` (`self.StaticMesh`) 0 "/Game/StudentWork/Materials/M_damage_flash.M_damage_flash" "None"))
  (set `self.FlashMaterial` _returnvalue))