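; Double sliding door actor that opens when something overlaps either of its two trigger components, Open or Open1, with no filter on the overlapping actor.
; MoveComponentTo slides the left and right panels apart over OpeningTime.
; Leaving either trigger closes the panels over ClosingTime after CloseDelay.
; A WalkedThrough flag blocks repeat openings until a short timer, started on overlap end, clears it.
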(event `self.Open1.OnComponentBeginOverlap`
  (params (OverlappedComponent :type "PrimitiveComponent Object Reference") (OtherActor :type "Actor Object Reference") (OtherComp :type "PrimitiveComponent Object Reference") (OtherBodyIndex :type Integer) (bFromSweep :type Boolean) (SweepResult :type "HitResult Structure (by ref)"))
  (if (not (`self.WalkedThrough`))
    (set `self.WalkedThrough` true)
    (`self.OpenDoor`)))

(event `self.Open.OnComponentBeginOverlap`
  (params (OverlappedComponent :type "PrimitiveComponent Object Reference") (OtherActor :type "Actor Object Reference") (OtherComp :type "PrimitiveComponent Object Reference") (OtherBodyIndex :type Integer) (bFromSweep :type Boolean) (SweepResult :type "HitResult Structure (by ref)"))
  (if (not (`self.WalkedThrough`))
    (set `self.WalkedThrough` true)
    (`self.OpenDoor`)))

(event `self.Open.OnComponentEndOverlap`
  (params (OverlappedComponent :type "PrimitiveComponent Object Reference") (OtherActor :type "Actor Object Reference") (OtherComp :type "PrimitiveComponent Object Reference") (OtherBodyIndex :type Integer))
  (`self.CLose Door`)
  (bind _returnvalue (`KismetSystemLibrary.K2_SetTimerDelegate` (delegate `WalkedThroughCooldown`) 0.2))
  (set `self.DoorCooldown` _returnvalue))

(event `OpenDoor`
  ; Open Door
  (`|ExecutionSequence`
    (:`then_0`
      (`KismetSystemLibrary.MoveComponentTo` (`self.DoorLeft`) (0.0 200.0 0.0) (struct) false false (`self.OpeningTime`)))
    (:`then_1`
      (`KismetSystemLibrary.MoveComponentTo` (`self.DoorRight`) (0.0 -400.0 0.0) (struct) false false (`self.OpeningTime`)))))

(event `WalkedThroughCooldown`
  (set `self.WalkedThrough` false))

(event `self.Open1.OnComponentEndOverlap`
  (params (OverlappedComponent :type "PrimitiveComponent Object Reference") (OtherActor :type "Actor Object Reference") (OtherComp :type "PrimitiveComponent Object Reference") (OtherBodyIndex :type Integer))
  (`self.Close Door`)
  (bind _returnvalue (`KismetSystemLibrary.K2_SetTimerDelegate` (delegate `WalkedThroughCooldown`) 0.2))
  (set `self.DoorCooldown2` _returnvalue))

(event `Close Door`
  ; Close Door
  (`KismetSystemLibrary.Delay` (`self.CloseDelay`))
  (`|ExecutionSequence`
    (:`then_0`
      (`KismetSystemLibrary.MoveComponentTo` (`self.DoorLeft`) (0.0 0.0 0.0) (struct) false false (`self.ClosingTime`)))
    (:`then_1`
      (`KismetSystemLibrary.MoveComponentTo` (`self.DoorRight`) (0.0 -200.0 0.0) (struct) false false (`self.ClosingTime`)))))

(fn `UserConstructionScript`)