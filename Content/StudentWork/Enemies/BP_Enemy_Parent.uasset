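; Base enemy class that detects the player, runs looping move and attack timers, and dies with an explosion.
; Move and Attack are empty events, presumably for children, alongside forward, random-yaw and player-aimed firing helpers.
; Tick turns the hull toward its velocity and, once RotateHead is set, aims the head at the player.
; Damage flashes the mesh red; death increments the room controller's death count and adds score to the player.
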(event `Aim at player`
  (bind _mytarget (`self.MyTarget`))
  (bind _head (`self.head`))
  ;[0.000427 0.01436 0.15 0.5] Aim at Player
  (if (`self.rotateHead`)
    (`/Engine/EditorBlueprintResources/StandardMacros.IsValid` _mytarget
      (:`Is Valid`
        (`SceneComponent.K2_SetWorldRotation` _head (`KismetMathLibrary.FindLookAtRotation` (`SceneComponent.K2_GetComponentLocation` _head) (`self.K2_GetActorLocation` _mytarget)) false false)))))

(event `Start Movement Timer`
  ;[0 0.01901 0.15 0.5] Movement Loop
  (bind _returnvalue (`KismetSystemLibrary.K2_SetTimerDelegate` (delegate `Move`) (`self.MovementUpdateTime`) true))
  (set `self.Movement Timer` _returnvalue))

(event `Move`
  ;[0 0.01901 0.15 0.5] Movement Loop
)

(event `HullToFace`
  (bind _returnvalue (`self.GetVelocity`))
  (bind _staticmesh (`self.StaticMesh`))
  (bind (_returnvalue_roll _returnvalue_pitch _returnvalue_yaw) (`KismetMathLibrary.BreakRotator` (`KismetMathLibrary.MakeRotFromX` _returnvalue)))
  ;[0.000444 0.006326 0.15 0.5] Smoth Hull Rotation
  (`/Engine/EditorBlueprintResources/StandardMacros.CompareFloat` (`KismetMathLibrary.VSize` _returnvalue)
    (:`>`
      (`SceneComponent.K2_SetWorldRotation` _staticmesh (`KismetMathLibrary.RInterpTo` (`SceneComponent.K2_GetComponentRotation` _staticmesh) (`KismetMathLibrary.MakeRotator` 0.0 0.0 _returnvalue_yaw) (`GameplayStatics.GetWorldDeltaSeconds`) 2.0) false false))))

(event `AddScore`
  (`/Game/Blueprints/BP_PlayerCharacter.UpdateScore` (`self.MyTarget`) (`self.Score`)))

(event `self.ReceiveBeginPlay`
  ; Set Variables
  (set `self.currentHealth` (`self.maxHealth`))
  (set `self.OriginalMaterial` (`PrimitiveComponent.GetMaterial` (`self.StaticMesh`) 0)))

(event `self.ReceiveTick`
  (params (DeltaSeconds :type "Float (single-precision)"))
  ; Event Tick
  (`self.Aim at player`)
  (`self.HullToFace`))

(event `BroadcastDeath`
  (bind _asroom_control_parent (cast `/Game/StudentWork/RoomControllers/RoomControlParent` (`self.RoomController`)))
  (set `/Game/StudentWork/RoomControllers/RoomControlParent.DeathsHad` (+ (`/Game/StudentWork/RoomControllers/RoomControlParent.DeathsHad` _asroom_control_parent) 1) _asroom_control_parent))

(event `Death Sequence`
  ;[0.15 0.006392 2.4e-05 0.5] Death Sequence
  (`NiagaraFunctionLibrary.SpawnSystemAtLocation` "/Game/StudentWork/Particles/NS_DeathExplosionv2.NS_DeathExplosionv2" (`SceneComponent.K2_GetComponentLocation` (`self.StaticMesh`)))
  (`self.BroadcastDeath`)
  (`self.AddScore`)
  (`self.K2_DestroyActor`))

(event `Start Attack Timer`
  ;[0.15 0 0 0.5] Attack Loop
  (bind _returnvalue (`KismetSystemLibrary.K2_SetTimerDelegate` (delegate `Attack`) (`self.Attack Speed`) true))
  (set `self.Attack Timer` _returnvalue))

(event `Attack`
  ;[0.15 0 0 0.5] Attack Loop
)

(event `self.ReceiveAnyDamage`
  (params (Damage :type "Float (single-precision)") (DamageType :type "DamageType Object Reference") (InstigatedBy :type "Controller Object Reference") (DamageCauser :type "Actor Object Reference"))
  ;[1 0.15 0.15 0.5] Take Damage
  (bind _output_get (set `self.currentHealth` (- (`self.currentHealth`) Damage)))
  (`PrimitiveComponent.CreateDynamicMaterialInstance` (`self.StaticMesh`) 0 "/Game/Materials/M_SciFi_Red.M_SciFi_Red" "None")
  (`/Engine/EditorBlueprintResources/StandardMacros.CompareFloat` _output_get
    (:`>`
      (`KismetSystemLibrary.Delay` 0.2)
      (`PrimitiveComponent.CreateDynamicMaterialInstance` (`self.StaticMesh`) 0 (`self.OriginalMaterial`) "None"))
    (:`==`
      (`self.Death Sequence` :!label _label))
    (:`<`
      (goto _label))))

(event `self.detection_radius.OnComponentBeginOverlap`
  (params (OverlappedComponent :type "PrimitiveComponent Object Reference") (OtherActor :type "Actor Object Reference") (OtherComp :type "PrimitiveComponent Object Reference") (OtherBodyIndex :type Integer) (bFromSweep :type Boolean) (SweepResult :type "HitResult Structure (by ref)"))
  ;[0.15 0.06728 0.000469 0.5] Player Detection
  (bind _asbp_player_character (cast `/Game/Blueprints/BP_PlayerCharacter` OtherActor))
  (set `self.MyTarget` _asbp_player_character)
  (`self.Start Movement Timer`)
  (`self.Start Attack Timer`))

(fn `ForwardFire`
  (params (Projectile :type "Actor Class Reference"))
  (bind _firearrow (`self.FireArrow`))
  (`/Engine/EditorBlueprintResources/StandardMacros.IsValid` (`self.MyTarget`)
    (:`Is Valid`
      (`|SpawnActorFromClass` Projectile (`KismetMathLibrary.MakeTransform` (`SceneComponent.K2_GetComponentLocation` _firearrow) (`SceneComponent.K2_GetComponentRotation` _firearrow)) "Undefined" "MultiplyWithRoot" null null))))

(fn `PlayerFire`
  (params (Projectile :type "Actor Class Reference"))
  (bind _mytarget (`self.MyTarget`))
  (bind _returnvalue (`SceneComponent.K2_GetComponentLocation` (`self.FireArrow`)))
  (`/Engine/EditorBlueprintResources/StandardMacros.IsValid` _mytarget
    (:`Is Valid`
      (set `self.rotateHead` true)
      (`|SpawnActorFromClass` Projectile (`KismetMathLibrary.MakeTransform` _returnvalue (`KismetMathLibrary.FindLookAtRotation` _returnvalue (`self.K2_GetActorLocation` _mytarget))) "Undefined" "MultiplyWithRoot" null null))))

(fn `RandomFire`
  (params (Projectile :type "Actor Class Reference"))
  (bind (_returnvalue_roll _returnvalue_pitch _returnvalue_yaw) (`KismetMathLibrary.BreakRotator` (`KismetMathLibrary.RandomRotator` false)))
  (`|SpawnActorFromClass` Projectile (`KismetMathLibrary.MakeTransform` (`SceneComponent.K2_GetComponentLocation` (`self.FireArrow`)) (`KismetMathLibrary.MakeRotator` 0.0 0.0 _returnvalue_yaw)) "Undefined" "MultiplyWithRoot" null null))

(fn `UserConstructionScript`)