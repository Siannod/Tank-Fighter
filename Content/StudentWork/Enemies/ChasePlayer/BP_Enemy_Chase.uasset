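; BP_Enemy_Chase is an enemy Blueprint that chases a target and fires projectiles.
; Its Move event uses AI MoveTo to approach MyTarget when valid, with an acceptance radius that stops it short of the target.
; Its Attack event spawns a BP_enemy_projectile at the FireArrow component's world location and rotation.
; Neither event is triggered within this graph, and the construction script only calls the parent's.
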(event `self.Move`
  (bind _mytarget (`self.MyTarget`))
  (`/Engine/EditorBlueprintResources/StandardMacros.IsValid` _mytarget
    (:`Is Valid`
      (`|AIMoveTo` self (0.0 0.0 0.0) _mytarget 300.0))))

(event `self.Attack`
  (bind _firearrow (`self.FireArrow`))
  (`|SpawnActorFromClass` "/Game/INACTIVE/OldWeapons/Projectiles/BP_enemy_projectile.BP_enemy_projectile_C" (`KismetMathLibrary.MakeTransform` (`SceneComponent.K2_GetComponentLocation` _firearrow) (`SceneComponent.K2_GetComponentRotation` _firearrow)) "Undefined" "MultiplyWithRoot" null null))

(fn `UserConstructionScript`
  (`parent.UserConstructionScript`))