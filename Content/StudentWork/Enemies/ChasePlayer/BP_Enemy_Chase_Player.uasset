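; BP_Enemy_Chase_Player is an enemy Blueprint that fires projectiles at its target.
; Its Attack event checks that MyTarget is valid, then spawns BP_enemy_projectile at the FireArrow component, rotated toward the target's location.
; The file holds no chase or attack-timing logic, BeginPlay and Tick are disabled, and MaxHealth and AttackSpeed are unused here.
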(event `self.Attack`
  (bind _mytarget (`self.MyTarget`))
  (bind _returnvalue (`SceneComponent.K2_GetComponentLocation` (`self.FireArrow`)))
  (`/Engine/EditorBlueprintResources/StandardMacros.IsValid` _mytarget
    (:`Is Valid`
      (`|SpawnActorFromClass` "/Game/StudentWork/Weapon/OldWeapons/Projectiles/BP_enemy_projectile.BP_enemy_projectile_C" (`KismetMathLibrary.MakeTransform` _returnvalue (`KismetMathLibrary.FindLookAtRotation` _returnvalue (`self.K2_GetActorLocation` _mytarget))) "Undefined" "MultiplyWithRoot" null null))))

(fn `UserConstructionScript`
  (`parent.UserConstructionScript`))