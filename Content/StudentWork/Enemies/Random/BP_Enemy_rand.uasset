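; BP_Enemy_rand is an enemy that moves to random points and fires projectiles.
; Its Move event sends it by AI MoveTo to a random reachable point within MoveRadius of its current location.
; Its Attack event spawns a BP_enemy_projectile at the FireArrow component's world location and rotation.
; Nothing in this graph calls either event, and the construction script only runs the parent's.
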(event `self.Move`
  (`|AIMoveTo` self (`NavigationSystemV1.K2_GetRandomReachablePointInRadius` (`self.K2_GetActorLocation`) (`self.moveRadius`) null null) null))

(event `self.Attack`
  (bind _firearrow (`self.FireArrow`))
  (`|SpawnActorFromClass` "/Game/StudentWork/Enemies/BP_enemy_projectile.BP_enemy_projectile_C" (`KismetMathLibrary.MakeTransform` (`SceneComponent.K2_GetComponentLocation` _firearrow) (`SceneComponent.K2_GetComponentRotation` _firearrow)) "Undefined" "MultiplyWithRoot" null null))

(fn `UserConstructionScript`
  (`parent.UserConstructionScript`))