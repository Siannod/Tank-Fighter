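; BP_RoomSix is a room controller that keeps the doors of its room locked until a required death count is reached.
; BeginPlay runs the parent logic, then clears AbleToOpen on every door in RoomDoors.
; Tick compares DeathsHad to DeathsNeeded and, once it is equal or greater, sets AbleToOpen on those doors every frame.
; The death count is only read here, never updated.
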(event `self.ReceiveBeginPlay`
  (`parent.ReceiveBeginPlay`)
  (for _array_element (`self.RoomDoors`)
    (set `/Game/StudentWork/BP_slidingDoor.ableToOpen` false _array_element)))

(event `self.ReceiveTick`
  (params (DeltaSeconds :type "Float (single-precision)"))
  (`/Engine/EditorBlueprintResources/StandardMacros.CompareInt` (`self.DeathsHad`) (`self.DeathsNeeded`)
    (:`>`
      _)
    (:`==`
      _))
  (for _array_element (`self.RoomDoors`)
    (set `/Game/StudentWork/BP_slidingDoor.ableToOpen` true _array_element)))

(fn `UserConstructionScript`
  (`parent.UserConstructionScript`))