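; BP_RoomSixA is a room controller that gates a set of sliding doors behind a death count.
; Overlapping its Box sets AbleToOpen to false on each BP_slidingDoor in the Doors array.
; Every Tick it compares DeathsHad with DeathsNeeded and, once the count is met or exceeded, re-enables all doors each frame, overriding the lock.
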(event `self.Box.OnComponentBeginOverlap`
  (params (OverlappedComponent :type "PrimitiveComponent Object Reference") (OtherActor :type "Actor Object Reference") (OtherComp :type "PrimitiveComponent Object Reference") (OtherBodyIndex :type Integer) (bFromSweep :type Boolean) (SweepResult :type "HitResult Structure (by ref)"))
  (for _array_element (`self.Doors`)
    (bind _asbp_sliding_door (cast `/Game/StudentWork/BP_slidingDoor` _array_element))
    (set `/Game/StudentWork/BP_slidingDoor.ableToOpen` false _asbp_sliding_door)))

(event `self.ReceiveTick`
  (params (DeltaSeconds :type "Float (single-precision)"))
  (`/Engine/EditorBlueprintResources/StandardMacros.CompareInt` (`self.DeathsHad`) (`self.DeathsNeeded`)
    (:`>`
      _)
    (:`==`
      _))
  (for _array_element (`self.Doors`)
    (set `/Game/StudentWork/BP_slidingDoor.ableToOpen` true _array_element)))

(fn `UserConstructionScript`
  (`parent.UserConstructionScript`))