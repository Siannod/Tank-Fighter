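; BP_roomFour is a room controller that unlocks the room four door once a required number of deaths is reached.
; Every Tick it compares DeathsHad with DeathsNeeded and, when they are equal, casts DoorReference to BP_RoomFourDour and sets its AbleToOpen flag.
; A failed cast prints "fail", and nothing in this Blueprint increments the death count itself.
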(event `self.ReceiveTick`
  (params (DeltaSeconds :type "Float (single-precision)"))
  (`/Engine/EditorBlueprintResources/StandardMacros.CompareInt` (`self.DeathsHad`) (`self.DeathsNeeded`)
    (:`==`
      (bind _asbp_room_four_dour (cast `/Game/StudentWork/BP_RoomFourDour` (`self.DoorReference`))
        (:`then`
          (set `/Game/StudentWork/BP_slidingDoor.ableToOpen` true _asbp_room_four_dour))
        (:`CastFailed`
          (`KismetSystemLibrary.PrintString` "fail"))))))

(fn `UserConstructionScript`
  (`parent.UserConstructionScript`))