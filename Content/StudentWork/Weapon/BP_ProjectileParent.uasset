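; Base projectile Blueprint for weapons that damages what it hits, then destroys itself with a Niagara effect.
; The static mesh hit event applies fixed damage to the hit actor and spawns NS_damage at the projectile's location.
; Separate PointDamage and AreaDamage functions offer parameterized single-target or radial damage with a chosen explosion effect.
; The hit event duplicates the point-damage logic inline, and neither function is called within this Blueprint.
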(event `self.StaticMesh.OnComponentHit`
  (params (HitComponent :type "PrimitiveComponent Object Reference") (OtherActor :type "Actor Object Reference") (OtherComp :type "PrimitiveComponent Object Reference") (NormalImpulse :type "Vector Structure") (Hit :type "HitResult Structure (by ref)"))
  (`GameplayStatics.ApplyDamage` OtherActor 10.0)
  (`self.K2_DestroyActor`)
  (`NiagaraFunctionLibrary.SpawnSystemAtLocation` "/Game/StudentWork/Particles/NS_damage.NS_damage" (`self.K2_GetActorLocation`)))

(fn `AreaDamage`
  (params (Damage :type "Float (double-precision)") (DamageRadius :type "Float (double-precision)") (CollisionExplosion :type "NiagaraSystem Object Reference"))
  (bind _returnvalue (`self.K2_GetActorLocation`))
  (`GameplayStatics.ApplyRadialDamage` :`BaseDamage` Damage :`Origin` _returnvalue :`DamageRadius` DamageRadius :`DamageCauser` null :`InstigatedByController` null)
  (`self.K2_DestroyActor`)
  (`NiagaraFunctionLibrary.SpawnSystemAtLocation` CollisionExplosion _returnvalue)
  (return))

(fn `PointDamage`
  (params (DamagedActor :type "Actor Object Reference") (Damage :type "Float (double-precision)") (CollisionExplosion :type "NiagaraSystem Object Reference"))
  (`GameplayStatics.ApplyDamage` DamagedActor Damage)
  (`self.K2_DestroyActor`)
  (`NiagaraFunctionLibrary.SpawnSystemAtLocation` CollisionExplosion (`self.K2_GetActorLocation`)))

(fn `UserConstructionScript`)