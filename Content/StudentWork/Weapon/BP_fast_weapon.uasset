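; BP_fast_weapon is a rapid-fire tank weapon that launches BP_fast_projectile actors when triggered.
; The Triggered event spawns each projectile at the location and rotation of the owning tank's DirectionArrow component.
; A Cooldown flag blocks further shots until a short timer calls EndCooldown, capping the fire rate at roughly ten shots per second.
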(event `self.Triggered`
  (bind _directionarrow (`/Game/Blueprints/BP_PlayerCharacter.DirectionArrow` (`self.MyTank`)))
  (if (not (`self.cooldown`))
    (`|SpawnActorFromClass` "/Game/StudentWork/Weapon/Projectiles/BP_fast_projectile.BP_fast_projectile_C" (`KismetMathLibrary.MakeTransform` (`SceneComponent.K2_GetComponentLocation` _directionarrow) (`SceneComponent.K2_GetComponentRotation` _directionarrow)) "Undefined" "MultiplyWithRoot" null null)
    (set `self.cooldown` true)
    (`KismetSystemLibrary.K2_SetTimerDelegate` (delegate `End Cooldown`) 0.1)))

(event `End Cooldown`
  (set `self.cooldown` false))

(fn `UserConstructionScript`
  (`parent.UserConstructionScript`))