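; Shotgun weapon Blueprint for a tank that fires three BP_Shotgun_Projectile actors per shot from the tank's DirectionArrow.
; One projectile flies straight and the other two get random yaw offsets in adjacent bands, so the spread fans to one side.
; Each shot uses a shell, and an empty magazine blocks firing until a timer refills it.
; A between-shot Cooldown flag is set and timer-cleared, but firing here checks only the reload flag.
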(event `self.Started`
  (bind _directionarrow (`/Game/Blueprints/BP_PlayerCharacter.DirectionArrow` (`self.MyTank`)))
  (bind _directionarrow_2 (`/Game/Blueprints/BP_PlayerCharacter.DirectionArrow` (`self.MyTank`)))
  (bind _directionarrow_3 (`/Game/Blueprints/BP_PlayerCharacter.DirectionArrow` (`self.MyTank`)))
  (if (not (`self.reload_cooldown`))
    (`|SpawnActorFromClass` "/Game/StudentWork/Weapon/Projectiles/BP_Shotgun_Projectile.BP_Shotgun_Projectile_C" (`KismetMathLibrary.MakeTransform` (`SceneComponent.K2_GetComponentLocation` _directionarrow_2) (`SceneComponent.K2_GetComponentRotation` _directionarrow_2)) "Undefined" "MultiplyWithRoot" null null)
    (`|SpawnActorFromClass` "/Game/StudentWork/Weapon/Projectiles/BP_Shotgun_Projectile.BP_Shotgun_Projectile_C" (`KismetMathLibrary.MakeTransform` (`SceneComponent.K2_GetComponentLocation` _directionarrow_3) (`KismetMathLibrary.ComposeRotators` (`SceneComponent.K2_GetComponentRotation` _directionarrow_3) (`KismetMathLibrary.MakeRotator` 0.0 0.0 (`KismetMathLibrary.Conv_IntToDouble` (`KismetMathLibrary.RandomIntegerInRange` 0 20))))) "Undefined" "MultiplyWithRoot" null null)
    (`|SpawnActorFromClass` "/Game/StudentWork/Weapon/Projectiles/BP_Shotgun_Projectile.BP_Shotgun_Projectile_C" (`KismetMathLibrary.MakeTransform` (`SceneComponent.K2_GetComponentLocation` _directionarrow) (`KismetMathLibrary.ComposeRotators` (`SceneComponent.K2_GetComponentRotation` _directionarrow) (`KismetMathLibrary.MakeRotator` 0.0 0.0 (`KismetMathLibrary.Conv_IntToDouble` (`KismetMathLibrary.RandomIntegerInRange` 20 40))))) "Undefined" "MultiplyWithRoot" null null)
    (bind _output_get (set `self.shells_left` (- (`self.shells_left`) 1)))
    (`/Engine/EditorBlueprintResources/StandardMacros.CompareInt` _output_get
      (:`>`
        (set `self.cooldown` true)
        (`KismetSystemLibrary.K2_SetTimerDelegate` (delegate `cooldown set`) 0.5))
      (:`==`
        (set `self.reload_cooldown` true :!label _label)
        (`KismetSystemLibrary.K2_SetTimerDelegate` (delegate `reolad`) 0.5))
      (:`<`
        (goto _label)))))

(event `cooldown set`
  (set `self.cooldown` false))

(event `reolad`
  (set `self.reload_cooldown` false)
  (set `self.shells_left` 2))

(fn `UserConstructionScript`
  (`parent.UserConstructionScript`))