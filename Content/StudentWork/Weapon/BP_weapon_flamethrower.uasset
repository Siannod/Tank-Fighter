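; Flamethrower weapon for a tank that deals area damage along the tank's DirectionArrow.
; Triggered runs a multi-sphere object trace forward from the arrow and damages each hit, throttled by a short timer-reset cooldown.
; Started spawns an attached Niagara flame once and reuses it, and Completed deactivates it.
; Tick also deactivates the flame when Pressed is false, though both Started and Completed set Pressed to true.
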(event `self.Triggered`
  (bind _directionarrow (`/Game/Blueprints/BP_PlayerCharacter.DirectionArrow` (`self.MyTank`)))
  (bind _returnvalue_location (`KismetMathLibrary.BreakTransform` (`SceneComponent.K2_GetComponentToWorld` _directionarrow)))
  (if (not (`self.Cooldown`))
    (bind _outhits (`KismetSystemLibrary.SphereTraceMultiForObjects` _returnvalue_location (+ _returnvalue_location (* (`SceneComponent.GetForwardVector` _directionarrow) (`self.Magnitude`))) 50.0 (`self.Object Types`)))
    (for _array_element _outhits
      (`GameplayStatics.ApplyDamage` (`.HitActor` (`GameplayStatics.BreakHitResult` _array_element)) 2.0))
    (set `self.Cooldown` true)
    (`KismetSystemLibrary.K2_SetTimerDelegate` (delegate `ResetCooldown`) 0.2)))

(event `ResetCooldown`
  (set `self.Cooldown` false))

(event `self.Started`
  (set `self.pressed` true)
  (`/Engine/EditorBlueprintResources/StandardMacros.IsValid` (`self.FlameSystem`)
    (:`Is Valid`
      (`ActorComponent.Activate` (`self.FlameSystem`) true))
    (:`Is Not Valid`
      (bind _returnvalue (`NiagaraFunctionLibrary.SpawnSystemAttached` "/Game/StudentWork/Particles/NS_flamer.NS_flamer" (`/Game/Blueprints/BP_PlayerCharacter.DirectionArrow` (`self.MyTank`)) "None" (0.0 0.0 0.0) (struct) "KeepRelativeOffset"))
      (set `self.FlameSystem` _returnvalue))))

(event `self.Completed`
  (bind _flamesystem (`self.FlameSystem`))
  (set `self.pressed` true)
  (`/Engine/EditorBlueprintResources/StandardMacros.IsValid` _flamesystem
    (:`Is Valid`
      (`ActorComponent.Deactivate` _flamesystem))))

(event `self.ReceiveTick`
  (params (DeltaSeconds :type "Float (single-precision)"))
  (`/Engine/EditorBlueprintResources/StandardMacros.IsValid` (`self.FlameSystem`)
    (:`Is Valid`
      (if (not (`self.pressed`))
        (`ActorComponent.Deactivate` (`self.FlameSystem`))))))

(fn `UserConstructionScript`
  (`parent.UserConstructionScript`))