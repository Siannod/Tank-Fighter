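; BP_FastWeapon is a rapid-fire tank weapon that shoots its own projectile with a light camera shake.
; When triggered outside a reload, a DoOnce gate passes the ammo check and cooldown state into the shared BasicFire function.
; A short timer then clears the cooldown and reopens the gate; triggering during a reload only restarts that cooldown.
; An older inline spawn-and-shake firing path remains, but its gate is never entered.
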(event `self.Triggered`
  (if (not (`self.Reloading`))
    (`/Engine/EditorBlueprintResources/StandardMacros.DoOnce` false :!label _label
      (:`Completed`
        (bind _noammo (`self.Check Ammo`))
        (`self.BasicFire` _noammo (`self.Cooldown`) "/Game/StudentWork/Weapon/FastWeapon/BP_FastWeapon_Projectile.BP_FastWeapon_Projectile_C" "/Game/StudentWork/Weapon/BP_cameraShake.BP_cameraShake_C" 0.25))))
  (set `self.Cooldown` true)
  (`KismetSystemLibrary.K2_SetTimerDelegate` (delegate `End Cooldown_1`) 0.15))

(event `End Cooldown_1`
  (set `self.Cooldown` false)
  (goto _label :!via `Reset`))

(event `self.EndCooldown`
  (bind _directionarrow (`/Game/Blueprints/BP_PlayerCharacter.DirectionArrow` (`self.MyTank`)))
  (set `self.Cooldown` false)
  (`/Engine/EditorBlueprintResources/StandardMacros.DoOnce` false :!via `Reset`
    (:`Completed`
      (bind _noammo (`self.Check Ammo`))
      (if _noammo
        (set `self.Cooldown` true :!label _label_2)
        (`KismetSystemLibrary.K2_SetTimerDelegate` (delegate `self.EndCooldown`) 0.3)
        (else
          (set `self.CurrentAmmo` (- (`self.CurrentAmmo`) 1))
          (if (not (`self.Cooldown`))
            (`|SpawnActorFromClass` "/Game/StudentWork/Weapon/FastWeapon/BP_FastWeapon_Projectile.BP_FastWeapon_Projectile_C" (`KismetMathLibrary.MakeTransform` (`SceneComponent.K2_GetComponentLocation` _directionarrow) (`SceneComponent.K2_GetComponentRotation` _directionarrow)) "Undefined" "MultiplyWithRoot" null null)
            (`self.CameraShake` "/Game/StudentWork/Weapon/BP_cameraShake.BP_cameraShake_C" 0.5)
            (goto _label_2)))))))

(fn `UserConstructionScript`
  (`parent.UserConstructionScript`))