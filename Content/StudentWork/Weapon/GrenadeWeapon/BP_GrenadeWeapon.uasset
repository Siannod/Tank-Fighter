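; Grenade weapon for a tank, with a hold-to-charge, release-to-fire shot.
; Triggered steadily raises FirePitch and updates the laser sight; Completed passes that pitch to BasicFire with the grenade projectile and camera shake.
; Firing also launches the tank opposite its laser sight as recoil, then resets pitch and sight.
; A DoOnce gate blocks further shots until a short timer clears the cooldown.
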(event `self.Completed`
  (`/Engine/EditorBlueprintResources/StandardMacros.DoOnce` false :!label _label
    (:`Completed`
      (`self.BasicFire` false (`self.Cooldown`) "/Game/StudentWork/Weapon/GrenadeWeapon/BP_GrenadeWeapon_Projectile.BP_GrenadeWeapon_Projectile_C" "/Game/StudentWork/Weapon/BP_cameraShake.BP_cameraShake_C" 0.0 (`self.Fire Pitch`))
      (`Character.LaunchCharacter` (`self.MyTank`) (* (`KismetMathLibrary.Normal` (`KismetMathLibrary.Conv_RotatorToVector` (`SceneComponent.K2_GetComponentRotation` (`/Game/Blueprints/BP_PlayerCharacter.LaserSight` (`self.MyTank`))))) -5000.0) false false)
      (set `self.Cooldown` true)
      (`self.SetLaserSight` 0.0)
      (set `self.Fire Pitch` 0.0)
      (`KismetSystemLibrary.K2_SetTimerDelegate` (delegate `self.EndCooldown`) 1.0))))

(event `self.EndCooldown`
  (set `self.Cooldown` false)
  (goto _label :!via `Reset`))

(event `self.Triggered`
  (bind _output_get (set `self.Fire Pitch` (+ (`self.Fire Pitch`) 0.3)))
  (`self.SetLaserSight` _output_get))

(fn `UserConstructionScript`
  (`parent.UserConstructionScript`))