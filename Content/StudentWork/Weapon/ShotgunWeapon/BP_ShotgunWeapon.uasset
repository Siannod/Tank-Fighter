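; Shotgun weapon for a tank that fires a burst of randomly scattered projectiles.
; On Completed, if CheckAmmo returns false, it spends one ammo for the whole burst.
; A loop spawns BP_ShotgunWeapon_Projectile actors at the tank's DirectionArrow, randomly offsetting pitch and yaw to form a cone-like spread.
; Each pellet spawn also triggers a light camera shake.
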(event `self.Completed`
  (bind _directionarrow (`/Game/Blueprints/BP_PlayerCharacter.DirectionArrow` (`self.MyTank`)))
  (bind (_returnvalue_roll _returnvalue_pitch _returnvalue_yaw) (`KismetMathLibrary.BreakRotator` (`SceneComponent.K2_GetComponentRotation` _directionarrow)))
  (bind _noammo (`self.Check Ammo`))
  (if (not _noammo)
    (set `self.CurrentAmmo` (- (`self.CurrentAmmo`) 1))
    (for _ (range 11)
      (`|SpawnActorFromClass` "/Game/StudentWork/Weapon/ShotgunWeapon/BP_ShotgunWeapon_Projectile.BP_ShotgunWeapon_Projectile_C" (`KismetMathLibrary.MakeTransform` (`SceneComponent.K2_GetComponentLocation` _directionarrow) (`KismetMathLibrary.MakeRotator` 0.0 (+ _returnvalue_pitch (`KismetMathLibrary.RandomFloatInRange` -20.0 20.0)) (+ _returnvalue_yaw (`KismetMathLibrary.RandomFloatInRange` -20.0 20.0)))) "Undefined" "MultiplyWithRoot" null null)
      (`self.CameraShake` "/Game/StudentWork/Weapon/BP_cameraShake.BP_cameraShake_C" 0.1))))

(fn `UserConstructionScript`
  (`parent.UserConstructionScript`))